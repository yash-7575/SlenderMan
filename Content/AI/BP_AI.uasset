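; AI-controlled melee character that detects the player and punches on demand.
; PawnSensing sets the seeingPlayer blackboard key for pawns tagged Player, while a looping timer periodically clears it.
; AttackPlayer plays a punch montage, guarded by an Attacking flag until completion.
; As the montage starts, it sphere-traces forward from AttackTracePoint with debug drawing and damages the hit pawn, without checking its tag.
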(event OnSeePawn(PawnSensing)
  (params (Pawn :type Pawn%20Object%20Reference))
  (if (Actor|ActorHasTag Pawn "Player")
    (AI|Components|Blackboard|SetValueasBool (AI|GetBlackboard (AI|GetAIController self)) (Utilities|Name|MakeLiteralName "seeingPlayer") true)))

(event Custom|Attack%20Player
  (bind _attack_trace_point (Variables|Default|GetAttack%20Trace%20Point))
  (bind _returnvalue (Transformation|GetWorldLocation _attack_trace_point))
  (if (not (Variables|Default|Getattacking?))
    (Variables|Default|Setattacking? true)
    (Animation|Montage|PlayMontage (Variables|Character|GetMesh) "/Game/AI/H2H_PunchCombo01_Montage.H2H_PunchCombo01_Montage"
      (:then
        (bind (_outhit _returnvalue_2) (Collision|SphereTraceForObjects _returnvalue (+ _returnvalue (* (Math|Vector|GetForwardVector (Transformation|GetWorldRotation _attack_trace_point)) 2e+02)) 5e+01 (Utilities|Array|MakeArray "ObjectTypeQuery3") false 0 "ForDuration"))
        (if _returnvalue_2
          (Game|Damage|ApplyDamage (.HitActor (Collision|BreakHitResult _outhit)) 1e+01 0 0)))
      (:OnCompleted
        (Variables|Default|Setattacking? false)))))

(event Custom|Stop%20Seeing%20Player
  (AI|Components|Blackboard|SetValueasBool (AI|GetBlackboard (AI|GetAIController self)) (Utilities|Name|MakeLiteralName "seeingPlayer") false))

(event EventBeginPlay
  (Utilities|Time|SetTimerbyEvent (delegate Custom|Stop%20Seeing%20Player) 0.8 true))

(fn ConstructionScript)